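; Enemy actor that damages the player when they touch its cube mesh.
; On overlap it casts to BP_Player and subtracts a fixed amount from the player's health.
; At zero health it flags the player dead and shows the restart display; otherwise it teleports the player a short distance along the world X axis.
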(event OnComponentBeginOverlap(Cube)
  (params (OverlappedComponent :type Primitive%20Component%20Object%20Reference) (OtherActor :type Actor%20Object%20Reference) (OtherComp :type Primitive%20Component%20Object%20Reference) (OtherBodyIndex :type Integer) (bFromSweep :type Boolean) (SweepResult :type Hit%20Result%20Structure%20%28by%20ref%29))
  ;[1 1 1] player got hit
  (Utilities|FlowControl|Sequence
    (:then_0
      (bind _asbp_player (Utilities|Casting|CastToBP_Player OtherActor))
      (Variables|Default|Setplayer _asbp_player)
      (Variables|/Game/InfiniteMatrix/Blueprints/BP_Player.BP_Player_C|Sethealth_left (Variables|Default|Getplayer) (- (Variables|/Game/InfiniteMatrix/Blueprints/BP_Player.BP_Player_C|Gethealth_left (Variables|Default|Getplayer)) 1e+01))
      (if (<= (Variables|/Game/InfiniteMatrix/Blueprints/BP_Player.BP_Player_C|Gethealth_left (Variables|Default|Getplayer)) 0.0)
        (Variables|/Game/InfiniteMatrix/Blueprints/BP_Player.BP_Player_C|SetIsDead (Variables|Default|Getplayer) true)
        (Default|DisplayRestart (Variables|Default|Getplayer))
        (else
          (Transformation|AddActorWorldOffset (Variables|Default|Getplayer) (Math|Vector|MakeVector 5e+01 0.0 0.0) false true))))))

(event EventBeginPlay)

(event Collision|EventActorBeginOverlap
  (params (OtherActor :type Actor%20Object%20Reference)))

(event EventTick
  (params (DeltaSeconds :type Float%20%28single-precision%29)))

(fn ConstructionScript)